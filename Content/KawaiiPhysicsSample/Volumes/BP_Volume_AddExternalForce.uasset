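; BP_Volume_AddExternalForce is a volume actor in the KawaiiPhysics sample that applies external forces to skeletal meshes while their actors are inside it.
; On Box begin overlap, it adds its ExternalForces to every skeletal mesh component of the entering actor, filtered by FilterTags with itself as owner.
; On end overlap, it removes the forces it owns from those components using the same tags.
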(event `self.Box.OnComponentBeginOverlap`
  (params (OverlappedComponent :type "PrimitiveComponent Object Reference") (OtherActor :type "Actor Object Reference") (OtherComp :type "PrimitiveComponent Object Reference") (OtherBodyIndex :type Integer) (bFromSweep :type Boolean) (SweepResult :type "HitResult Structure (by ref)"))
  (for _array_element (`self.K2_GetComponentsByClass` OtherActor "/Script/Engine.SkeletalMeshComponent")
    (`KawaiiPhysicsLibrary.AddExternalForcesToComponent` _array_element (`self.External Forces`) self (`self.Filter Tags`))))

(event `self.Box.OnComponentEndOverlap`
  (params (OverlappedComponent :type "PrimitiveComponent Object Reference") (OtherActor :type "Actor Object Reference") (OtherComp :type "PrimitiveComponent Object Reference") (OtherBodyIndex :type Integer))
  (for _array_element (`self.K2_GetComponentsByClass` OtherActor "/Script/Engine.SkeletalMeshComponent")
    (`KawaiiPhysicsLibrary.RemoveExternalForcesFromComponent` _array_element self (`self.Filter Tags`))))

(fn `UserConstructionScript`)